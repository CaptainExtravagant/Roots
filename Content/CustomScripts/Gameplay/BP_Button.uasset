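; BP_Button is an overlap-triggered button that activates and deactivates a list of linked actors.
; Overlapping the Box plays a timeline that slides the Button mesh by an offset, reversing once the Box is empty.
; When the timeline finishes, its direction selects Pressed or Released, which sends ActivateMessage or DeactivateMessage to each valid actor in TriggeredActors.
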(event `self.ReceiveBeginPlay`
  (set `self.ButtonStart` (`SceneComponent.RelativeLocation` (`self.Button`))))

(event `self.Box.OnComponentBeginOverlap`
  (params (OverlappedComponent :type "PrimitiveComponent Object Reference") (OtherActor :type "Actor Object Reference") (OtherComp :type "PrimitiveComponent Object Reference") (OtherBodyIndex :type Integer) (bFromSweep :type Boolean) (SweepResult :type "HitResult Structure (by ref)"))
  (bind _buttonstart (`self.ButtonStart`))
  (bind (_direction _alpha) (`Timeline|T_Press` :!label _label)
    (:`Update`
      (`SceneComponent.K2_SetRelativeLocation` (`self.Button`) (`KismetMathLibrary.VLerp` _buttonstart (+ _buttonstart (`self.ButtonOffset`)) _alpha) false false))
    (:`Finished`
      (if (`|EnumEquality` _direction "Forward")
        (`self.Pressed`)
        (else
          (`self.Released`))))))

(event `self.Box.OnComponentEndOverlap`
  (params (OverlappedComponent :type "PrimitiveComponent Object Reference") (OtherActor :type "Actor Object Reference") (OtherComp :type "PrimitiveComponent Object Reference") (OtherBodyIndex :type Integer))
  (if (<= (`KismetArrayLibrary.Array_Length` (`PrimitiveComponent.GetOverlappingActors` (`self.Box`) null)) 0)
    (goto _label :!via `Reverse`)))

(event `Pressed`
  (`KismetSystemLibrary.PrintString` "Button Pressed")
  (for _array_element (`self.TriggeredActors`)
    (`/Engine/EditorBlueprintResources/StandardMacros.IsValid` _array_element
      (:`Is Valid`
        (message `/Game/CustomScripts/Interfaces/I_Interact.Activate` _array_element)))))

(event `Released`
  (`KismetSystemLibrary.PrintString` "Button Released")
  (for _array_element (`self.TriggeredActors`)
    (`/Engine/EditorBlueprintResources/StandardMacros.IsValid` _array_element
      (:`Is Valid`
        (message `/Game/CustomScripts/Interfaces/I_Interact.Deactivate` _array_element)))))

(fn `UserConstructionScript`)