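; BP_Cable is an interactable cable obstacle that the player breaks by pulling.
; Interact grabs its Box with the character's PhysicsHandle, and Tick then compares the Box's world Y offset from its start against CableThreshold.
; BreakCable detaches cable ends, releases and destroys the grab components, restores orient-to-movement, disables BlockingVolume collision and calls ActivateMessage on TrappedActors.
; The distance-scaled cable force logic is disconnected.
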(event `self.ReceiveBeginPlay`
  (set `self.DefaultCableForce` (`CableComponent.CableForce` (`self.Cable_Left`)))
  (set `self.BoxDefault` (`SceneComponent.K2_GetComponentLocation` (`self.Box`))))

(event `self.ReceiveTick`
  (params (DeltaSeconds :type "Float (single-precision)"))
  (bind _cablethreshold (`self.CableThreshold`))
  (bind (_boxdefault_x _boxdefault_y) (`KismetMathLibrary.BreakVector` (`self.BoxDefault`)))
  (bind (_returnvalue_x _returnvalue_y) (`KismetMathLibrary.BreakVector` (`SceneComponent.K2_GetComponentLocation` (`self.Box`))))
  (bind _returnvalue (- _boxdefault_y _returnvalue_y))
  (if (`self.Grabbed`)
    (if (or (>= _returnvalue _cablethreshold) (<= _returnvalue (* _cablethreshold -1.0)))
      (`self.BreakCable`))))

(event `BreakCable`
  (bind _interacting_character (`self.Interacting Character`))
  (set `self.Grabbed` false)
  (for _array_element (`self.K2_GetComponentsByClass` "/Script/CableComponent.CableComponent")
    (set `CableComponent.bAttachEnd` false _array_element))
  (`PhysicsHandleComponent.ReleaseComponent` (`/Game/CustomScripts/PlayerCharacter/C_BaseCharacter.PhysicsHandle` _interacting_character))
  (`ActorComponent.K2_DestroyComponent` (`self.Box`))
  (`ActorComponent.K2_DestroyComponent` (`self.CableGrab`))
  (set `CharacterMovementComponent.bOrientRotationToMovement` true (`Character.CharacterMovement` _interacting_character))
  (`PrimitiveComponent.SetCollisionEnabled` (`self.BlockingVolume`) "NoCollision")
  (for _array_element_2 (`self.TrappedActors`)
    (`/Engine/EditorBlueprintResources/StandardMacros.IsValid` _array_element_2
      (:`Is Valid`
        (message `/Game/CustomScripts/Interfaces/I_Interact.Activate` _array_element_2)))))

(event `/Game/CustomScripts/Interfaces/I_Interact.Interact`
  (params (InteractingCharacter :type "/Game/CustomScripts/PlayerCharacter/C_BaseCharacter Object Reference"))
  (`KismetSystemLibrary.PrintString` "Interacted")
  (`PhysicsHandleComponent.GrabComponentAtLocation` (`/Game/CustomScripts/PlayerCharacter/C_BaseCharacter.PhysicsHandle` InteractingCharacter) (`self.Box`) "None" (`self.K2_GetActorLocation` InteractingCharacter))
  (set `self.Grabbed` true)
  (set `self.Interacting Character` InteractingCharacter))

(fn `UserConstructionScript`)