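; BP_TutorialSign is a tutorial sign that flickers on the first time something overlaps its trigger box.
; On BeginPlay it creates dynamic materials for the instruction and two half-circle components and sets their LightStrength to zero.
; The first overlap plays a timeline whose event tracks switch the light on, then set the materials' FlickerSpeed to settle the flicker.
; The overlap does not filter which actor triggers it.
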(event `self.ReceiveBeginPlay`
  (bind _halfcircle1 (`self.HalfCircle1`))
  (bind _instruction (`self.Instruction`))
  (bind _halfcircle (`self.HalfCircle`))
  (bind _returnvalue (`PrimitiveComponent.CreateDynamicMaterialInstance` _halfcircle1 0 (`PrimitiveComponent.GetMaterial` _halfcircle1 0) "None"))
  (set `self.DynamicMaterial1` _returnvalue)
  (bind _returnvalue_2 (`PrimitiveComponent.CreateDynamicMaterialInstance` _instruction 0 (`PrimitiveComponent.GetMaterial` _instruction 0) "None"))
  (set `self.DynamicMaterial2` _returnvalue_2)
  (bind _returnvalue_3 (`PrimitiveComponent.CreateDynamicMaterialInstance` _halfcircle 0 (`PrimitiveComponent.GetMaterial` _halfcircle 0) "None"))
  (set `self.DynamicMaterial3` _returnvalue_3)
  (`MaterialInstanceDynamic.SetScalarParameterValue` (`self.DynamicMaterial1`) "LightStrength" 0.0)
  (`MaterialInstanceDynamic.SetScalarParameterValue` (`self.DynamicMaterial2`) "LightStrength" 0.0)
  (`MaterialInstanceDynamic.SetScalarParameterValue` (`self.DynamicMaterial3`) "LightStrength" 0.0))

(event `self.Box.OnComponentBeginOverlap`
  (params (OverlappedComponent :type "PrimitiveComponent Object Reference") (OtherActor :type "Actor Object Reference") (OtherComp :type "PrimitiveComponent Object Reference") (OtherBodyIndex :type Integer) (bFromSweep :type Boolean) (SweepResult :type "HitResult Structure (by ref)"))
  (`/Engine/EditorBlueprintResources/StandardMacros.DoOnce` false
    (:`Completed`
      (`Timeline|T_FlickerOn`
        (:`TurnOn`
          (`MaterialInstanceDynamic.SetScalarParameterValue` (`self.DynamicMaterial1`) "LightStrength" 1.0)
          (`MaterialInstanceDynamic.SetScalarParameterValue` (`self.DynamicMaterial2`) "LightStrength" 1.0)
          (`MaterialInstanceDynamic.SetScalarParameterValue` (`self.DynamicMaterial3`) "LightStrength" 1.0))
        (:`FlickerSettle`
          (`MaterialInstanceDynamic.SetScalarParameterValue` (`self.DynamicMaterial3`) "FlickerSpeed" 1.0)
          (`MaterialInstanceDynamic.SetScalarParameterValue` (`self.DynamicMaterial2`) "FlickerSpeed" 1.0)
          (`MaterialInstanceDynamic.SetScalarParameterValue` (`self.DynamicMaterial1`) "FlickerSpeed" 1.0))))))

(fn `UserConstructionScript`)