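; BP_ElectricTrap is an electric trap hazard that deals a fixed amount of damage to any actor that begins overlapping its box.
; Activate and Deactivate events switch the trap on and off by toggling the box between query-only and no collision.
; The same events show or hide the two static meshes, so visibility matches whether the trap can deal damage.
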(event `self.Box.OnComponentBeginOverlap`
  (params (OverlappedComponent :type "PrimitiveComponent Object Reference") (OtherActor :type "Actor Object Reference") (OtherComp :type "PrimitiveComponent Object Reference") (OtherBodyIndex :type Integer) (bFromSweep :type Boolean) (SweepResult :type "HitResult Structure (by ref)"))
  (`GameplayStatics.ApplyDamage` OtherActor 100.0))

(event `/Game/CustomScripts/Interfaces/I_Interact.Activate`
  (`PrimitiveComponent.SetCollisionEnabled` (`self.Box`) "QueryOnly")
  (`SceneComponent.SetVisibility` (`self.StaticMesh1`) true false)
  (`SceneComponent.SetVisibility` (`self.StaticMesh`) true false))

(event `/Game/CustomScripts/Interfaces/I_Interact.Deactivate`
  (`PrimitiveComponent.SetCollisionEnabled` (`self.Box`) "NoCollision")
  (`SceneComponent.SetVisibility` (`self.StaticMesh1`) false false)
  (`SceneComponent.SetVisibility` (`self.StaticMesh`) false false))

(fn `UserConstructionScript`)