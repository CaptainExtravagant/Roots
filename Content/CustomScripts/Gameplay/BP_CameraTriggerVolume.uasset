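; Trigger volume that switches the game camera to a scenario camera state while a base character is inside its box.
; It caches BP_GameCamera on BeginPlay, then on overlap passes itself as the scenario camera with a configurable blend time.
; Leaving the box restores the other camera state with zero blend time.
; Two cross-resetting DoOnce gates keep repeated overlap events from re-triggering the same switch.
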(event `self.ReceiveBeginPlay`
  (bind _returnvalue (`GameplayStatics.GetActorOfClass` "/Game/CustomScripts/BP_GameCamera.BP_GameCamera_C"))
  (set `self.GameCamera` _returnvalue))

(event `self.Box.OnComponentBeginOverlap`
  (params (OverlappedComponent :type "PrimitiveComponent Object Reference") (OtherActor :type "Actor Object Reference") (OtherComp :type "PrimitiveComponent Object Reference") (OtherBodyIndex :type Integer) (bFromSweep :type Boolean) (SweepResult :type "HitResult Structure (by ref)"))
  (cast `/Game/CustomScripts/PlayerCharacter/C_BaseCharacter` OtherActor)
  (`|ExecutionSequence`
    (:`then_0`
      (`/Engine/EditorBlueprintResources/StandardMacros.DoOnce` false :!label _label
        (:`Completed`
          (`/Game/CustomScripts/BP_GameCamera.ChangeState` (`self.GameCamera`) "NewEnumerator1" self (`self.Blend Time`)))))
    (:`then_1`
      (goto _label_2 :!via `Reset`))))

(event `self.Box.OnComponentEndOverlap`
  (params (OverlappedComponent :type "PrimitiveComponent Object Reference") (OtherActor :type "Actor Object Reference") (OtherComp :type "PrimitiveComponent Object Reference") (OtherBodyIndex :type Integer))
  (cast `/Game/CustomScripts/PlayerCharacter/C_BaseCharacter` OtherActor)
  (`|ExecutionSequence`
    (:`then_0`
      (goto _label :!via `Reset`))
    (:`then_1`
      (`/Engine/EditorBlueprintResources/StandardMacros.DoOnce` false :!label _label_2
        (:`Completed`
          (`/Game/CustomScripts/BP_GameCamera.ChangeState` (`self.GameCamera`) "NewEnumerator0" null 0.0))))))

(fn `UserConstructionScript`)