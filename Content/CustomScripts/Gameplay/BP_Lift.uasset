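; BP_Lift is a lift actor that moves its static mesh between its starting world position and an end offset.
; A timeline, with play rate derived from LiftTime and optional looping, lerps the mesh position as it plays or reverses.
; Activate and Deactivate set delayed timer events, guarded by an active flag.
; A looping lift ignores Deactivate.
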(event `self.ReceiveBeginPlay`
  (bind _t_lift (`self.T_Lift`))
  (`TimelineComponent.SetLooping` _t_lift (`self.ShouldLoop`))
  (`TimelineComponent.SetPlayRate` _t_lift (/ 1.0 (`self.LiftTime`)))
  (set `self.StartPosition` (`SceneComponent.K2_GetComponentLocation` (`self.StaticMesh`))))

(event `StartLift`
  (bind _startposition (`self.StartPosition`))
  (bind (_direction _alpha) (`Timeline|T_Lift` :!label _label)
    (:`Update`
      (`SceneComponent.K2_SetWorldLocation` (`self.StaticMesh`) (`KismetMathLibrary.VLerp` _startposition (+ _startposition (`self.EndOffset`)) _alpha) false false))))

(event `StopLift`
  (goto _label :!via `Reverse`))

(event `/Game/CustomScripts/Interfaces/I_Interact.Activate`
  (if (not (`self.IsActive`))
    (bind _returnvalue (`KismetSystemLibrary.K2_SetTimerDelegate` (`|CreateDelegate` :!event `StartLift`) (`self.Delay`)))
    (set `self.LiftTimerHandle` _returnvalue)
    (set `self.IsActive` true)))

(event `/Game/CustomScripts/Interfaces/I_Interact.Deactivate`
  (if (and (`self.IsActive`) (not (`self.ShouldLoop`)))
    (bind _returnvalue (`KismetSystemLibrary.K2_SetTimerDelegate` (`|CreateDelegate` :!event `StopLift`) (`self.Delay`)))
    (set `self.LiftTimerHandle` _returnvalue)
    (set `self.IsActive` false)))

(fn `UserConstructionScript`)