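; BP_NPC is a talkable NPC that shows an alert popup and a dialogue widget, currently filled with Lorem ipsum placeholder text.
; A C_BaseCharacter entering InteractOverlap plays the popup once, and Interact prints the dialogue.
; When the last overlapping actor leaves, the popup reverses and re-arms, and any printed dialogue is hidden through a DoOnce that Interact resets.
; An unconnected random-greeting PrintString remains unused.
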(event `self.ReceiveBeginPlay`
  (bind _asw_alert (cast `/Game/CustomScripts/Widgets/W_Alert` (`WidgetComponent.GetWidget` (`self.AlertWidget`))))
  (`UserWidget.PlayAnimation` _asw_alert (`/Game/CustomScripts/Widgets/W_Alert.Popup` _asw_alert) 0.0 1 "Reverse" 1.0 false)
  (bind _asw_dialogue (cast `/Game/CustomScripts/Widgets/W_Dialogue` (`WidgetComponent.GetWidget` (`self.DialogueWidget`))))
  (`/Game/CustomScripts/Widgets/W_Dialogue.UpdateDialogue` _asw_dialogue "Lorem ipsum dolor sit amet, consectetur adipiscing elit, sed do eiusmod tempor incididunt ut labore et dolore magna aliqua. Ut enim ad minim veniam, quis nostrud exercitation ullamco laboris nisi ut aliquip ex ea commodo consequat. Duis aute irure dolor in reprehenderit in voluptate velit esse cillum dolore eu fugiat nulla pariatur. Excepteur sint occaecat cupidatat non proident, sunt in culpa qui officia deserunt mollit anim id est laborum."))

(event `self.InteractOverlap.OnComponentBeginOverlap`
  (params (OverlappedComponent :type "PrimitiveComponent Object Reference") (OtherActor :type "Actor Object Reference") (OtherComp :type "PrimitiveComponent Object Reference") (OtherBodyIndex :type Integer) (bFromSweep :type Boolean) (SweepResult :type "HitResult Structure (by ref)"))
  (cast `/Game/CustomScripts/PlayerCharacter/C_BaseCharacter` OtherActor)
  (`/Engine/EditorBlueprintResources/StandardMacros.DoOnce` false :!label _label
    (:`Completed`
      (bind _asw_alert (cast `/Game/CustomScripts/Widgets/W_Alert` (`WidgetComponent.GetWidget` (`self.AlertWidget`))))
      (`UserWidget.PlayAnimation` _asw_alert (`/Game/CustomScripts/Widgets/W_Alert.Popup` _asw_alert) 0.0 1 "Forward" 2.0 false))))

(event `self.InteractOverlap.OnComponentEndOverlap`
  (params (OverlappedComponent :type "PrimitiveComponent Object Reference") (OtherActor :type "Actor Object Reference") (OtherComp :type "PrimitiveComponent Object Reference") (OtherBodyIndex :type Integer))
  (cast `/Game/CustomScripts/PlayerCharacter/C_BaseCharacter` OtherActor)
  (if (<= (`KismetArrayLibrary.Array_Length` (`PrimitiveComponent.GetOverlappingActors` (`self.InteractOverlap`) null)) 0)
    (`|ExecutionSequence`
      (:`then_0`
        (goto _label :!via `Reset`))
      (:`then_1`
        (bind _asw_alert (cast `/Game/CustomScripts/Widgets/W_Alert` (`WidgetComponent.GetWidget` (`self.AlertWidget`))))
        (`UserWidget.PlayAnimation` _asw_alert (`/Game/CustomScripts/Widgets/W_Alert.Popup` _asw_alert) 0.0 1 "Reverse" 1.0 false))
      (:`then_2`
        (`/Engine/EditorBlueprintResources/StandardMacros.DoOnce` true :!label _label_2
          (:`Completed`
            (bind _asw_dialogue (cast `/Game/CustomScripts/Widgets/W_Dialogue` (`WidgetComponent.GetWidget` (`self.DialogueWidget`))))
            (`/Game/CustomScripts/Widgets/W_Dialogue.HideDialogue` _asw_dialogue)))))))

(event `/Game/CustomScripts/Interfaces/I_Interact.Interact`
  (params (InteractingCharacter :type "/Game/CustomScripts/PlayerCharacter/C_BaseCharacter Object Reference"))
  (bind _asw_dialogue (cast `/Game/CustomScripts/Widgets/W_Dialogue` (`WidgetComponent.GetWidget` (`self.DialogueWidget`))))
  (`/Game/CustomScripts/Widgets/W_Dialogue.PrintDialogue` _asw_dialogue)
  (goto _label_2 :!via `Reset`))

(fn `UserConstructionScript`)