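; BP_Lever is a three-position lever that players grab to switch two sets of trigger actors on and off.
; Interact attaches the Handle to the interacting character's PhysicsHandle.
; Tick converts the handle's relative roll into left, right or neutral.
; On each change it sends DeactivateMessage to the previous side's actors and ActivateMessage to the new side's, with neutral activating none.
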(event `self.ReceiveTick`
  (params (DeltaSeconds :type "Float (single-precision)"))
  (bind _relativerotation_roll (`KismetMathLibrary.BreakRotator` (`SceneComponent.RelativeRotation` (`self.Handle`))))
  (if (< _relativerotation_roll -25.0)
    (if (!= (`self.SwitchPosition`) 1)
      (`self.ResetSwitch`)
      (set `self.SwitchPosition` 1)
      (`self.SwitchUpdated` :!label _label))
    (elif (> _relativerotation_roll 25.0)
      (if (!= (`self.SwitchPosition`) 2)
        (`self.ResetSwitch`)
        (set `self.SwitchPosition` 2)
        (goto _label))
      (elif (!= (`self.SwitchPosition`) 0)
        (`self.ResetSwitch`)
        (set `self.SwitchPosition` 0)
        (goto _label)))))

(event `/Game/CustomScripts/Interfaces/I_Interact.Interact`
  (params (InteractingCharacter :type "/Game/CustomScripts/PlayerCharacter/C_BaseCharacter Object Reference"))
  (`PhysicsHandleComponent.GrabComponentAtLocation` (`/Game/CustomScripts/PlayerCharacter/C_BaseCharacter.PhysicsHandle` InteractingCharacter) (`self.Handle`) "None" (`self.K2_GetActorLocation` InteractingCharacter))
  (`KismetSystemLibrary.PrintString` "Interacted"))

(event `SwitchUpdated`
  (`/Engine/EditorBlueprintResources/StandardMacros.DoOnce` false :!label _label_2
    (:`Completed`
      (for _array_element (select `int` (`self.SwitchPosition`) :`0` _ :`1` (`self.LeftTriggerActors`) :`2` (`self.RightTriggerActors`))
        (`/Engine/EditorBlueprintResources/StandardMacros.IsValid` _array_element
          (:`Is Valid`
            (message `/Game/CustomScripts/Interfaces/I_Interact.Activate` _array_element)))))))

(event `ResetSwitch`
  (for _array_element (select `int` (`self.SwitchPosition`) :`0` _ :`1` (`self.LeftTriggerActors`) :`2` (`self.RightTriggerActors`))
    (`/Engine/EditorBlueprintResources/StandardMacros.IsValid` _array_element
      (:`Is Valid`
        (message `/Game/CustomScripts/Interfaces/I_Interact.Deactivate` _array_element))))
  (goto _label_2 :!via `Reset`))

(fn `UserConstructionScript`)