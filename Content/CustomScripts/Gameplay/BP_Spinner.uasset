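; Spinner Blueprint that rotates through a RotatingMovement component and can be switched on and off.
; StartActive sets whether it begins at full yaw speed or stationary.
; Activate and Deactivate play and reverse a timeline that lerps the rotation rate, easing the spin up and down.
; A pair of DoOnce gates that reset each other ignores repeated calls in the same state.
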(event `self.ReceiveBeginPlay`
  (bind _rotatingmovement (`self.RotatingMovement`))
  (if (`self.StartActive`)
    (set `RotatingMovementComponent.RotationRate` (`KismetMathLibrary.MakeRotator` 0.0 180.0) _rotatingmovement)
    (else
      (set `RotatingMovementComponent.RotationRate` (`KismetMathLibrary.MakeRotator` 0.0 0.0) _rotatingmovement))))

(event `/Game/CustomScripts/Interfaces/I_Interact.Activate`
  (`|ExecutionSequence`
    (:`then_0`
      (`/Engine/EditorBlueprintResources/StandardMacros.DoOnce` (`self.StartActive`) :!label _label
        (:`Completed`
          (bind (_direction _alpha) (`Timeline|T_StartSpeed` :!label _label_2)
            (:`Update`
              (set `RotatingMovementComponent.RotationRate` (`KismetMathLibrary.MakeRotator` 0.0 (`KismetMathLibrary.Lerp` 0.0 180.0 _alpha)) (`self.RotatingMovement`)))))))
    (:`then_1`
      (goto _label_3 :!via `Reset`))))

(event `/Game/CustomScripts/Interfaces/I_Interact.Deactivate`
  (`|ExecutionSequence`
    (:`then_0`
      (`/Engine/EditorBlueprintResources/StandardMacros.DoOnce` false :!label _label_3
        (:`Completed`
          (goto _label_2 :!via `Reverse`))))
    (:`then_1`
      (goto _label :!via `Reset`))))

(fn `UserConstructionScript`)