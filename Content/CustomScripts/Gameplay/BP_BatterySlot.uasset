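; Battery slot actor that powers a list of triggered actors while a BP_Battery sits inside its box.
; An overlapping battery, including one already present at BeginPlay, sends ActivateMessage to every TriggeredActor and turns two point lights green.
; A battery entering during play also receives ActivateMessage itself.
; A battery leaving sends DeactivateMessage to the triggered actors and turns the lights red.
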(event `self.ReceiveBeginPlay`
  (for _array_element (`PrimitiveComponent.GetOverlappingActors` (`self.Box`) null)
    (cast `/Game/CustomScripts/Gameplay/BP_Battery` _array_element)
    (for _array_element_2 (`self.TriggeredActors`) :!label _label
      (`/Engine/EditorBlueprintResources/StandardMacros.IsValid` _array_element_2
        (:`Is Valid`
          (message `/Game/CustomScripts/Interfaces/I_Interact.Activate` _array_element_2))))
    (`LightComponent.SetLightColor` (`self.PointLight`) (struct :`G` 1.0 :`B` 0.001442 :`A` 1.0) true)
    (`LightComponent.SetLightColor` (`self.PointLight1`) (struct :`G` 1.0 :`B` 0.001442 :`A` 1.0) true)))

(event `self.Box.OnComponentBeginOverlap`
  (params (OverlappedComponent :type "PrimitiveComponent Object Reference") (OtherActor :type "Actor Object Reference") (OtherComp :type "PrimitiveComponent Object Reference") (OtherBodyIndex :type Integer) (bFromSweep :type Boolean) (SweepResult :type "HitResult Structure (by ref)"))
  (bind _asbp_battery (cast `/Game/CustomScripts/Gameplay/BP_Battery` OtherActor))
  (message `/Game/CustomScripts/Interfaces/I_Interact.Activate` _asbp_battery)
  (goto _label))

(event `self.Box.OnComponentEndOverlap`
  (params (OverlappedComponent :type "PrimitiveComponent Object Reference") (OtherActor :type "Actor Object Reference") (OtherComp :type "PrimitiveComponent Object Reference") (OtherBodyIndex :type Integer))
  (cast `/Game/CustomScripts/Gameplay/BP_Battery` OtherActor)
  (for _array_element (`self.TriggeredActors`)
    (`/Engine/EditorBlueprintResources/StandardMacros.IsValid` _array_element
      (:`Is Valid`
        (message `/Game/CustomScripts/Interfaces/I_Interact.Deactivate` _array_element))))
  (`LightComponent.SetLightColor` (`self.PointLight`) (struct :`R` 1.0 :`A` 1.0) true)
  (`LightComponent.SetLightColor` (`self.PointLight1`) (struct :`R` 1.0 :`A` 1.0) true))

(fn `UserConstructionScript`)