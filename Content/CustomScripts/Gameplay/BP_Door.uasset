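; BP_Door is a door actor that swings between a closed and an open rotation when activated or deactivated.
; Activate and Deactivate open or close it immediately, or set a one-shot timer when the matching delay is positive.
; The T_Open timeline lerps the actor's rotation, playing forward to open and reversing to close.
; BeginPlay either calls Activate when StartOpen is set or snaps the door to its closed rotation.
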(event `/Game/CustomScripts/Interfaces/I_Interact.Activate`
  (bind _opendelay (`self.OpenDelay`))
  (if (> _opendelay 0.0)
    (bind _returnvalue (`KismetSystemLibrary.K2_SetTimerDelegate` (`|CreateDelegate` :!event `OpenDoor`) _opendelay))
    (set `self.DelayTimer` _returnvalue)
    (else
      (`self.OpenDoor`))))

(event `self.ReceiveBeginPlay`
  (if (`self.StartOpen`)
    (`/Game/CustomScripts/Interfaces/I_Interact.Activate`)
    (else
      (`self.K2_SetActorRotation` (`self.ClosedRotation`)))))

(event `OpenDoor`
  (bind (_direction _alpha) (`Timeline|T_Open` :!label _label)
    (:`Update`
      (`self.K2_SetActorRotation` (`KismetMathLibrary.RLerp` (`self.ClosedRotation`) (`self.OpenRotation`) _alpha)))))

(event `/Game/CustomScripts/Interfaces/I_Interact.Deactivate`
  (bind _closedelay (`self.CloseDelay`))
  (if (> _closedelay 0.0)
    (bind _returnvalue (`KismetSystemLibrary.K2_SetTimerDelegate` (`|CreateDelegate` :!event `CloseDoor`) _closedelay))
    (set `self.DelayTimer` _returnvalue)
    (else
      (`self.CloseDoor`))))

(event `CloseDoor`
  (goto _label :!via `Reverse`))

(fn `UserConstructionScript`)