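; BP_GameCamera is the game camera, switching between following the characters and handing the view to a scenario camera.
; While following, Tick eases its Y and Z toward the average location of all C_BaseCharacter actors, leaving X untouched.
; ChangeState blends the player's view to itself or the supplied scenario camera, opening or closing a gate that controls the follow update.
; BeginPlay opens that gate, so following runs from the start.
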(event `self.ReceiveTick`
  (params (DeltaSeconds :type "Float (single-precision)"))
  (bind (_returnvalue_x _returnvalue_y _returnvalue_z) (`KismetMathLibrary.BreakVector` (`self.K2_GetActorLocation`)))
  (bind _delta_seconds (`self.Delta Seconds`))
  (set `self.Delta Seconds` DeltaSeconds)
  (`/Engine/EditorBlueprintResources/StandardMacros.Gate` true :!label _label
    (:`Exit`
      (bind _outactors (`GameplayStatics.GetAllActorsOfClass` "/Game/CustomScripts/PlayerCharacter/C_BaseCharacter.C_BaseCharacter_C"))
      (if (> (`KismetArrayLibrary.Array_Length` _outactors) 0)
        (bind _returnvalue (`GameplayStatics.GetActorArrayAverageLocation` _outactors))
        (`self.K2_SetActorLocation` (`KismetMathLibrary.MakeVector` 0.0 (`KismetMathLibrary.FInterpTo` _returnvalue_y (.y _returnvalue) _delta_seconds 1.5) (`KismetMathLibrary.FInterpTo` _returnvalue_z (.z _returnvalue) _delta_seconds 1.5)))))))

(event `self.ReceiveBeginPlay`
  (goto _label :!via `Open`))

(event `ChangeState`
  (params (NewState :type "/Game/CustomScripts/E_CameraState Enum" :default "NewEnumerator0") (ScenarioCamera :type "Actor Object Reference") (BlendTime :type "Float (double-precision)"))
  (bind _returnvalue (`GameplayStatics.GetPlayerController` 0))
  (bind _output_get (set `self.CurrentState` NewState))
  (switch `/Game/CustomScripts/E_CameraState` _output_get
    (:`NewEnumerator0`
      (`PlayerController.SetViewTargetWithBlend` _returnvalue self 1.0 "VTBlend_EaseInOut" 2.0 true)
      (goto _label :!via `Open`))
    (:`NewEnumerator1`
      (`PlayerController.SetViewTargetWithBlend` _returnvalue ScenarioCamera BlendTime "VTBlend_EaseInOut" 1.0 true)
      (goto _label :!via `Close`))))

(fn `UserConstructionScript`)