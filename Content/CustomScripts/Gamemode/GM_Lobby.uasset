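; Lobby game mode that handles drop-in joining for local multiplayer on a shared camera.
; On BeginPlay it points the first player's view at the BP_GameCamera, pre-creates local players and binds to each PC_Lobby's join event.
; On join, it records the controller and uses its join index to pick a named player start and a blue, green, red or yellow material for the spawned, unpossessed character.
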(event `self.ReceiveBeginPlay`
  (`|ExecutionSequence`
    (:`then_0`
      (bind _returnvalue (`GameplayStatics.GetActorOfClass` "/Game/CustomScripts/BP_GameCamera.BP_GameCamera_C"))
      (bind _output_get (set `self.GameCam` _returnvalue))
      (`PlayerController.SetViewTargetWithBlend` (`GameplayStatics.GetPlayerController` 0) _output_get 0.0 "VTBlend_Linear" 0.0 false))
    (:`then_1`
      (for _ (range 4)
        (bind _returnvalue_2 (`GameplayStatics.CreatePlayer` -1))
        (bind _aspc_lobby (cast `/Game/CustomScripts/PlayerCharacter/PC_Lobby` _returnvalue_2))
        (add `/Game/CustomScripts/PlayerCharacter/PC_Lobby.PlayerJoin` _aspc_lobby (delegate `OnPlayerJoin`))))))

(event `OnPlayerJoin`
  (params (JoinedPlayer :type "/Game/CustomScripts/PlayerCharacter/PC_Lobby Object Reference"))
  (bind _returnvalue (`KismetArrayLibrary.Array_Add` (`self.ActiveControllers`) JoinedPlayer))
  (bind _returnvalue_2 (`|SpawnActorFromClass` "/Game/CustomScripts/PlayerCharacter/C_BaseCharacter.C_BaseCharacter_C" (`self.GetTransform` (`self.K2_FindPlayerStart` JoinedPlayer (`KismetStringLibrary.Conv_IntToString` _returnvalue))) "AlwaysSpawn" "OverrideRootScale" null null))
  (`PrimitiveComponent.SetMaterial` (`Character.Mesh` _returnvalue_2) 0 (select `int` _returnvalue :`0` "/Game/CustomAssets/Materials/Characters/MI_Character_Blue.MI_Character_Blue" :`1` "/Game/CustomAssets/Materials/Characters/MI_Character_Green.MI_Character_Green" :`2` "/Game/CustomAssets/Materials/Characters/MI_Character_Red.MI_Character_Red" :`3` "/Game/CustomAssets/Materials/Characters/MI_Character_Yellow.MI_Character_Yellow" :!type "MaterialInterface Object Reference")))

(fn `UserConstructionScript`)