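; BP_RespawnPoint is a respawn point with a limited number of charges, shown on a counter widget.
; On BeginPlay it stores its capsule's transform as SpawnTransform and initializes the W_RespawnCounter with the current charges.
; A Character overlapping the capsule fires TriggerActive, passing the point itself.
; ReduceCharges always ticks the widget down, then spends a charge if any remain and returns whether it did.
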(event `self.ReceiveBeginPlay`
  (set `self.SpawnTransform` (`SceneComponent.K2_GetComponentToWorld` (`self.Capsule`)))
  (bind _asw_respawn_counter (cast `/Game/CustomScripts/Widgets/W_RespawnCounter` (`WidgetComponent.GetWidget` (`self.CounterWidget`))))
  (bind _output_get (set `self.WidgetRef` _asw_respawn_counter))
  (`/Game/CustomScripts/Widgets/W_RespawnCounter.SetupSpawnCount` _output_get (`self.CurrentCharges`)))

(event `self.Capsule.OnComponentBeginOverlap`
  (params (OverlappedComponent :type "PrimitiveComponent Object Reference") (OtherActor :type "Actor Object Reference") (OtherComp :type "PrimitiveComponent Object Reference") (OtherBodyIndex :type Integer) (bFromSweep :type Boolean) (SweepResult :type "HitResult Structure (by ref)"))
  (cast `Character` OtherActor)
  (`KismetSystemLibrary.PrintString` "SpawnTriggered")
  (`self.TriggerActive` self))

(fn `ReduceCharges`
  (returns (Success :type Boolean))
  (`/Game/CustomScripts/Widgets/W_RespawnCounter.TickDown` (`self.WidgetRef`))
  (if (> (`self.CurrentCharges`) 0)
    (`/Engine/EditorBlueprintResources/StandardMacros.DecrementInt` (`self.CurrentCharges`)
      (:`  `
        (return true)))
    (else
      (return false))))

(fn `UserConstructionScript`)