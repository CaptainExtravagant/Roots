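; BP_LevelEnd is a level exit trigger that ends the current level when a C_BaseCharacter overlaps its box.
; The first valid overlap prints a completion message and fades the player camera and audio out, holding the faded screen.
; A one-shot timer then opens the NextLevel reference a few seconds later, after the fade finishes.
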(event `self.Box.OnComponentBeginOverlap`
  (params (OverlappedComponent :type "PrimitiveComponent Object Reference") (OtherActor :type "Actor Object Reference") (OtherComp :type "PrimitiveComponent Object Reference") (OtherBodyIndex :type Integer) (bFromSweep :type Boolean) (SweepResult :type "HitResult Structure (by ref)"))
  (cast `/Game/CustomScripts/PlayerCharacter/C_BaseCharacter` OtherActor)
  (`/Engine/EditorBlueprintResources/StandardMacros.DoOnce` false
    (:`Completed`
      (`KismetSystemLibrary.PrintString` "Level Complete")
      (`PlayerCameraManager.StartCameraFade` :`self` (`PlayerController.PlayerCameraManager` (`GameplayStatics.GetPlayerController` 0)) :`ToAlpha` 1.0 :`Duration` 3.0 :`bShouldFadeAudio` true :`bHoldWhenFinished` true)
      (bind _returnvalue (`KismetSystemLibrary.K2_SetTimerDelegate` (delegate `ChangeLevel`) 5.0))
      (set `self.LevelChangeTimerHandle` _returnvalue))))

(event `ChangeLevel`
  (`GameplayStatics.OpenLevelBySoftObjectPtr` (`self.NextLevel`)))

(fn `UserConstructionScript`)